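; BP_Health is a health pickup that heals the player when collected.
; Its Collect event casts player character 0 to Sci_Fi_ShooterCharacter, calls Heal with a fixed amount, then destroys the pickup.
; If the cast fails, the pickup stays in the world.
; Collect's trigger lies outside this graph, as the overlap, BeginPlay and Tick events are disabled.
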(event EventBeginPlay
  (|CallParentFunction) ; This node is disabled and will not be called.\nDrag off pins to build functionality.
)

(event Collision|EventActorBeginOverlap
  (params (OtherActor :type Actor%20Object%20Reference))
  (|CallParentFunction OtherActor) ; This node is disabled and will not be called.\nDrag off pins to build functionality.
)

(event EventTick
  (params (DeltaSeconds :type Float%20%28single-precision%29))
  (|CallParentFunction DeltaSeconds) ; This node is disabled and will not be called.\nDrag off pins to build functionality.
)

(event EventCollect
  (bind _assci_fi_shooter_character (Utilities|Casting|CastToSci_Fi_ShooterCharacter (Game|GetPlayerCharacter 0)))
  (Class|SciFiShooterCharacter|Heal _assci_fi_shooter_character 0.0 2e+01)
  (Actor|DestroyActor))

(fn ConstructionScript
  (|CallParentFunction))